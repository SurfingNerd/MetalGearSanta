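; Player Santa character who sneaks past sleeping dogs to deliver a present to the Christmas tree.
; Camera-relative input moves Santa, Sneak halves it, and Tick wakes listed dogs when input speed is high.
; Holding Action near the tree fills a progress bar that resets if interrupted and spawns the parcel once full.
; Death and win events show pausing screens; paused Tick throttles axis-driven navigation of the game-over menu.
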(event Custom|OnWin
  (bind _returnvalue (Game|GetPlayerController 0))
  (bind _returnvalue_2 (UserInterface|CreateWidget "/Game/Blueprints/UI/WT_WinScreen.WT_WinScreen_C"))
  (UserInterface|Viewport|AddtoViewport _returnvalue_2 0)
  (Variables|/Script/Engine.PlayerController|SetbShowMouseCursor _returnvalue true)
  (Input|SetInputModeGameandUI _returnvalue _returnvalue_2 "LockOnCapture" false)
  (Game|SetGamePaused true))

(event Custom|OnDeath
  (bind _returnvalue (Game|GetPlayerController 0))
  (bind _returnvalue_2 (UserInterface|CreateWidget "/Game/Blueprints/UI/WT_GameOverScreen.WT_GameOverScreen_C"))
  (UserInterface|Viewport|AddtoViewport _returnvalue_2 0)
  (Variables|/Script/Engine.PlayerController|SetbShowMouseCursor _returnvalue true)
  (Input|SetInputModeGameandUI _returnvalue _returnvalue_2 "LockOnCapture" false)
  (Game|SetGamePaused true)
  (Variables|Default|SetGameOverScreen _returnvalue_2))

(event EventTick
  (params (DeltaSeconds :type Float%20%28single-precision%29))
  (bind _xmastree (Variables|Default|GetXMasTree))
  (if (Game|IsGamePaused)
    (CallFunction|UITick DeltaSeconds)
    (else
      (Utilities|FlowControl|Sequence
        (:then_0
          (if (>= (Variables|Default|GetSpeed) 0.8)
            (for _array_element (Variables|Default|GetSleepingDogs)
              (Default|WakeUp _array_element (Transformation|GetActorLocation)))))
        (:then_1
          (if (and (not (Variables|Default|GetHasDeliveredPresent)) (Variables|Default|GetIsPlacing))
            (bind _output_get (Variables|Default|SetPresentPlacement (+ (Variables|Default|GetPresentPlacement) DeltaSeconds)))
            (bind _aswt_progressbar (Utilities|Casting|CastToWT_Progressbar (UserInterface|GetUserWidgetObject (Variables|Default|GetProgressBar))))
            (Progress|SetPercent (Variables|/Game/Blueprints/UI/WT_Progressbar.WT_Progressbar_C|GetProgressBar_0 _aswt_progressbar) (/ _output_get 3.0))
            (if (>= (/ _output_get 3.0) 1.0)
              (Variables|Default|SetHasDeliveredPresent true)
              (Rendering|SetVisibility (Variables|Default|GetProgressBar) false false)
              (Utilities|IsValid _xmastree
                (:Is%20Valid
                  (Default|SpawnParcel _xmastree))))
            (else
              (Variables|Default|SetPresentPlacement 0.0)
              (bind _aswt_progressbar_2 (Utilities|Casting|CastToWT_Progressbar (UserInterface|GetUserWidgetObject (Variables|Default|GetProgressBar))))
              (Progress|SetPercent (Variables|/Game/Blueprints/UI/WT_Progressbar.WT_Progressbar_C|GetProgressBar_0 _aswt_progressbar_2) 0.0))))))))

(event Input|ActionEvents|InputActionSneak
  (params (Key :type Key%20Structure))
  (:Pressed
    (Variables|Default|SetSneaking true))
  (:Released
    (Variables|Default|SetSneaking false)))

(event Input|ActionEvents|InputActionAction
  (params (Key :type Key%20Structure))
  (:Pressed
    (if (Variables|Default|GetIsNearTree)
      (Variables|Default|SetIsPlacing true)))
  (:Released
    (Variables|Default|SetIsPlacing false)))

(event Input|AxisEvents|InputAxisMoveForward
  (params (AxisValue :type Float%20%28single-precision%29))
  (bind _returnvalue (Pawn|GetControlRotation :!class /Script/Engine.Pawn))
  (bind _returnvalue_2 (Transformation|GetActorLocation))
  (bind _pitch (Math|Rotator|BreakRotator _returnvalue))
  (bind _returnvalue_3 (Math|Rotator|MakeRotator 0.0 _pitch 0.0))
  (bind _returnvalue_4 (Math|Vector|GetForwardVector _returnvalue_3))
  (if (Variables|Default|GetSneaking)
    (Variables|Default|SetForwardValue (* AxisValue 0.5))
    (else
      (Variables|Default|SetForwardValue AxisValue)))
  (Pawn|Input|AddMovementInput _returnvalue_4 (Variables|Default|GetForwardValue) false)
  (Variables|Default|SetSpeed (Math|Vector|VectorLength (+ (* _returnvalue_4 (Variables|Default|GetForwardValue)) (* (Math|Vector|GetRightVector _returnvalue_3) (Variables|Default|GetRightValue)))))
  (Transformation|SetWorldRotation (Variables|Default|GetSantaMesh) (Math|Rotator|FindLookatRotation _returnvalue_2 (+ _returnvalue_2 (+ (* _returnvalue_4 (Variables|Default|GetForwardValue)) (* (Math|Vector|GetRightVector _returnvalue_3) (Variables|Default|GetRightValue))))) false false))

(event Input|AxisEvents|InputAxisMoveRight
  (params (AxisValue :type Float%20%28single-precision%29))
  (if (Variables|Default|GetSneaking)
    (Variables|Default|SetRightValue (* AxisValue 0.5))
    (else
      (Variables|Default|SetRightValue AxisValue)))
  (Pawn|Input|AddMovementInput (Math|Vector|GetRightVector (Math|Rotator|MakeRotator 0.0 (.Pitch (Math|Rotator|BreakRotator (Pawn|GetControlRotation :!class /Script/Engine.Pawn))) 0.0)) (Variables|Default|GetRightValue) false))

(event Custom|UITick
  (params (DeltaSeconds :type Float%20%28single-precision%29))
  (if (> (Variables|UI|GetInputTime) 0.0)
    (Variables|UI|SetInputTime (- (Variables|UI|GetInputTime) DeltaSeconds))))

(event Input|ActionEvents|InputActionConfirm
  (params (Key :type Key%20Structure))
  (bind _gameoverscreen (Variables|Default|GetGameOverScreen))
  (:Pressed
    (Utilities|IsValid _gameoverscreen
      (:Is%20Valid
        (Default|PressedConfirm _gameoverscreen)))))

(event Input|AxisEvents|InputAxisMoveForward
  (params (AxisValue :type Float%20%28single-precision%29))
  (Utilities|IsValid (Variables|Default|GetGameOverScreen)
    (:Is%20Valid
      (if (<= (Variables|UI|GetInputTime) 0.0)
        (if (> AxisValue (Variables|UI|GetInputOffset))
          (Default|PressedUp (Variables|Default|GetGameOverScreen))
          (Variables|UI|SetInputTime (Variables|UI|GetInputDelay))
          (elif (< AxisValue (* -1 (Variables|UI|GetInputOffset)))
            (Default|PressedDown (Variables|Default|GetGameOverScreen))
            (Variables|UI|SetInputTime (Variables|UI|GetInputDelay))))))))

(fn ConstructionScript)