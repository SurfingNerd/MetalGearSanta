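; BP_BGM plays background music, resuming from the position saved in BP_GameInstance so it survives this Blueprint being recreated.
; On BeginPlay it adds the last playback percent, scaled by BGMSound's duration, to the previous start time, subtracting the duration if it overruns.
; It plays Audio from that offset and stores it as the new BGMTime.
; The playback-percent event continually writes progress back to the game instance.
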(event OnAudioPlaybackPercent(Audio)
  (params (PlayingSoundWave :type Sound%20Wave%20Object%20Reference) (PlaybackPercent :type Float%20%28single-precision%29))
  (Variables|/Game/Blueprints/GameMode/BP_GameInstance.BP_GameInstance_C|SetBGMPercent (Variables|Default|GetGameInstance) PlaybackPercent))

(event EventBeginPlay
  (bind _bgm_sound (Variables|Default|GetBGM_Sound))
  (bind _duration (Variables|/Script/Engine.SoundBase|GetDuration _bgm_sound))
  (bind _asbp_game_instance (Utilities|Casting|CastToBP_GameInstance (Game|GetGameInstance)))
  (Variables|Default|SetGameInstance _asbp_game_instance)
  (Utilities|FlowControl|Sequence
    (:then_0
      (if (> (+ (* _duration (Variables|/Game/Blueprints/GameMode/BP_GameInstance.BP_GameInstance_C|GetBGMPercent (Variables|Default|GetGameInstance))) (Variables|/Game/Blueprints/GameMode/BP_GameInstance.BP_GameInstance_C|GetBGMTime (Variables|Default|GetGameInstance))) _duration)
        (Variables|Default|SetNewBGMTime (- (+ (* _duration (Variables|/Game/Blueprints/GameMode/BP_GameInstance.BP_GameInstance_C|GetBGMPercent (Variables|Default|GetGameInstance))) (Variables|/Game/Blueprints/GameMode/BP_GameInstance.BP_GameInstance_C|GetBGMTime (Variables|Default|GetGameInstance))) _duration))
        (else
          (Variables|Default|SetNewBGMTime (+ (* _duration (Variables|/Game/Blueprints/GameMode/BP_GameInstance.BP_GameInstance_C|GetBGMPercent (Variables|Default|GetGameInstance))) (Variables|/Game/Blueprints/GameMode/BP_GameInstance.BP_GameInstance_C|GetBGMTime (Variables|Default|GetGameInstance)))))))
    (:then_1
      (Audio|Components|Audio|Play (Variables|Default|GetAudio) (Variables|Default|GetNewBGMTime))
      (Variables|/Game/Blueprints/GameMode/BP_GameInstance.BP_GameInstance_C|SetBGMTime (Variables|Default|GetGameInstance) (Variables|Default|GetNewBGMTime)))))

(fn ConstructionScript)