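; BP_Dog is an enemy dog that can sleep, be woken by noise, and kill Santa.
; While it sleeps, Santa entering its box registers it in his SleepingDogs list, and leaving removes it.
; WakeUp clears the sleep state, writes the noise location to the AI blackboard and removes it from the game mode's SleepingEnemies.
; Tick derives IsMoving from velocity, and KillSanta calls OnDeath on the stored Santa.
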(event OnComponentBeginOverlap(Box)
  (params (OverlappedComponent :type Primitive%20Component%20Object%20Reference) (OtherActor :type Actor%20Object%20Reference) (OtherComp :type Primitive%20Component%20Object%20Reference) (OtherBodyIndex :type Integer) (bFromSweep :type Boolean) (SweepResult :type Hit%20Result%20Structure%20%28by%20ref%29))
  (if (Variables|Default|GetIsSleeping)
    (bind _asbp_santa (Utilities|Casting|CastToBP_Santa OtherActor))
    (bind _output_get (Variables|Default|SetSanta _asbp_santa))
    (Utilities|Array|Add (Variables|/Game/Blueprints/Santa/BP_Santa.BP_Santa_C|GetSleepingDogs _output_get) self)))

(event OnComponentEndOverlap(Box)
  (params (OverlappedComponent :type Primitive%20Component%20Object%20Reference) (OtherActor :type Actor%20Object%20Reference) (OtherComp :type Primitive%20Component%20Object%20Reference) (OtherBodyIndex :type Integer))
  (bind _asbp_santa (Utilities|Casting|CastToBP_Santa OtherActor))
  (Utilities|Array|RemoveItem (Variables|/Game/Blueprints/Santa/BP_Santa.BP_Santa_C|GetSleepingDogs _asbp_santa) self))

(event Custom|KillSanta
  (bind _santa (Variables|Default|GetSanta))
  (Utilities|IsValid _santa
    (:Is%20Valid
      (Default|OnDeath _santa))))

(event EventBeginPlay)

(event Collision|EventActorBeginOverlap
  (params (OtherActor :type Actor%20Object%20Reference)))

(event EventTick
  (params (DeltaSeconds :type Float%20%28single-precision%29))
  (if (and (!= (Math|Vector|VectorLength (Variables|/Script/Engine.MovementComponent|GetVelocity (Variables|Character|GetCharacterMovement))) 0.0) (not (Variables|Default|GetIsMoving)))
    (Variables|Default|SetIsMoving true)
    (elif (and (Variables|Default|GetIsMoving) (== (Math|Vector|VectorLength (Variables|/Script/Engine.MovementComponent|GetVelocity (Variables|Character|GetCharacterMovement))) 0.0))
      (Variables|Default|SetIsMoving false))))

(event EventWakeUp
  (params (NoiseLocation :type Vector :default "0, 0, 0"))
  (bind _returnvalue (Utilities|Name|MakeLiteralName "NoiseLocation"))
  (bind _returnvalue_2 (AI|GetBlackboard 0))
  (Variables|Default|SetIsSleeping false)
  (Utilities|IsValid (AI|Components|Blackboard|GetValueasObject _returnvalue_2 _returnvalue)
    (:Is%20Not%20Valid
      (AI|Components|Blackboard|SetValueasVector _returnvalue_2 _returnvalue NoiseLocation)
      (bind _asbp_metal_gear_santa_gm (Utilities|Casting|CastToBP_MetalGearSantaGM (Game|GetGameMode)))
      (Utilities|Array|RemoveItem (Variables|/Game/Blueprints/GameMode/BP_MetalGearSantaGM.BP_MetalGearSantaGM_C|GetSleepingEnemies _asbp_metal_gear_santa_gm) self))))

(fn ConstructionScript)