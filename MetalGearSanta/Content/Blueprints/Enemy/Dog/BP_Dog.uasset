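; BP_Dog is an enemy dog that sleeps until woken and can kill Santa.
; A Box overlap tracks Santa and adds or removes the dog from Santa's SleepingDogs list, with debug prints.
; WakeUp clears IsSleeping and, if the Blackboard's Santa object is unset, writes the tracked Santa there for the AI.
; KillSanta calls OnDeath on the tracked Santa if valid.
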(event OnComponentBeginOverlap(Box)
  (params (OverlappedComponent :type Primitive%20Component%20Object%20Reference) (OtherActor :type Actor%20Object%20Reference) (OtherComp :type Primitive%20Component%20Object%20Reference) (OtherBodyIndex :type Integer) (bFromSweep :type Boolean) (SweepResult :type Hit%20Result%20Structure%20%28by%20ref%29))
  (bind _asbp_santa (Utilities|Casting|CastToBP_Santa OtherActor))
  (bind _output_get (Variables|Default|SetSanta _asbp_santa))
  (Utilities|Array|Add (Variables|/Game/Blueprints/Santa/BP_Santa.BP_Santa_C|GetSleepingDogs _output_get) self)
  (Development|PrintString "Remove")
  (Development|PrintString (Utilities|String|ToString(Integer) (Utilities|Array|Length (Variables|/Game/Blueprints/Santa/BP_Santa.BP_Santa_C|GetSleepingDogs _output_get)))))

(event OnComponentEndOverlap(Box)
  (params (OverlappedComponent :type Primitive%20Component%20Object%20Reference) (OtherActor :type Actor%20Object%20Reference) (OtherComp :type Primitive%20Component%20Object%20Reference) (OtherBodyIndex :type Integer))
  (bind _asbp_santa (Utilities|Casting|CastToBP_Santa OtherActor))
  (Variables|Default|SetSanta 0)
  (Utilities|Array|RemoveItem (Variables|/Game/Blueprints/Santa/BP_Santa.BP_Santa_C|GetSleepingDogs _asbp_santa) self)
  (Development|PrintString "Remove")
  (Development|PrintString (Utilities|String|ToString(Integer) (Utilities|Array|Length (Variables|/Game/Blueprints/Santa/BP_Santa.BP_Santa_C|GetSleepingDogs _asbp_santa)))))

(event Custom|KillSanta
  (bind _santa (Variables|Default|GetSanta))
  (Utilities|IsValid _santa
    (:Is%20Valid
      (Default|OnDeath _santa))))

(event Custom|WakeUp
  (bind _returnvalue (Utilities|Name|MakeLiteralName "Santa"))
  (bind _returnvalue_2 (AI|GetBlackboard 0))
  (Variables|Default|SetIsSleeping false)
  (Utilities|IsValid (AI|Components|Blackboard|GetValueasObject _returnvalue_2 _returnvalue)
    (:Is%20Not%20Valid
      (AI|Components|Blackboard|SetValueasBool _returnvalue_2 _returnvalue false)
      (AI|Components|Blackboard|SetValueasObject _returnvalue_2 _returnvalue (Variables|Default|GetSanta)))))

(event EventBeginPlay)

(event Collision|EventActorBeginOverlap
  (params (OtherActor :type Actor%20Object%20Reference)))

(event EventTick
  (params (DeltaSeconds :type Float%20%28single-precision%29)))

(fn ConstructionScript)