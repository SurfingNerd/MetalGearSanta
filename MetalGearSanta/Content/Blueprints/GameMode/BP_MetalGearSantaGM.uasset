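; Game mode for MetalGearSanta that tracks sleeping enemies and wakes them in response to a noise.
; BeginPlay caches all actors implementing the BP_Enemy interface and all BP_ChildWaypoint actors.
; WakeAllUp stores the noise location, loops over the cached enemies and casts each to BP_Dog to call WakeUp with that location, so only dogs respond.
; The waypoint list is stored but not used within this graph.
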(event Custom|WakeAllUp
  (params (NoiseLocation :type Vector))
  (Variables|Default|SetNoiseLocation NoiseLocation)
  (for _array_element (Variables|Default|GetSleepingEnemies)
    (bind _asbp_dog (Utilities|Casting|CastToBP_Dog _array_element))
    (Default|WakeUp _asbp_dog (Variables|Default|GetNoiseLocation))))

(event EventBeginPlay
  (bind _outactors (Actor|GetAllActorswithInterface "/Game/Blueprints/Enemy/BP_Enemy.BP_Enemy_C"))
  (Variables|Default|SetSleepingEnemies _outactors)
  (bind _outactors_2 (Actor|GetAllActorsOfClass "/Game/Blueprints/Enemy/Child/BP_ChildWaypoint.BP_ChildWaypoint_C"))
  (Variables|Default|SetChildWaypoints _outactors_2))

(event EventTick
  (params (DeltaSeconds :type Float%20%28single-precision%29)))

(fn ConstructionScript)