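; Player Santa character who delivers a present while sneaking past sleeping dogs.
; Movement inputs, halved while sneaking, drive directions built from control pitch only, mesh facing and a Speed value that wakes listed dogs when high.
; Holding Action, begun near the tree, fills a progress-bar widget on Tick until delivery, resetting on release.
; OnWin and OnDeath (also triggered by a P key shortcut) show end screens and pause the game.
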(event Custom|OnWin
  (bind _returnvalue (UserInterface|CreateWidget "/Game/Blueprints/UI/WT_WinScreen.WT_WinScreen_C"))
  (UserInterface|Viewport|AddtoViewport _returnvalue 0)
  (Variables|/Script/Engine.PlayerController|SetbShowMouseCursor (Game|GetPlayerController 0) true)
  (Game|SetGamePaused true))

(event Custom|OnDeath
  (bind _returnvalue (UserInterface|CreateWidget "/Game/Blueprints/UI/WT_GameOverScreen.WT_GameOverScreen_C"))
  (UserInterface|Viewport|AddtoViewport _returnvalue 0)
  (Variables|/Script/Engine.PlayerController|SetbShowMouseCursor (Game|GetPlayerController 0) true)
  (Game|SetGamePaused true))

(event EventBeginPlay)

(event Collision|EventActorBeginOverlap
  (params (OtherActor :type Actor%20Object%20Reference)))

(event EventTick
  (params (DeltaSeconds :type Float%20%28single-precision%29))
  (Utilities|FlowControl|Sequence
    (:then_0
      (if (>= (Variables|Default|GetSpeed) 0.7)
        (for _array_element (Variables|Default|GetSleepingDogs)
          (Default|WakeUp _array_element (Transformation|GetActorLocation)))))
    (:then_1
      (if (and (not (Variables|Default|GetHasDeliveredPresent)) (Variables|Default|GetIsPlacing))
        (bind _output_get (Variables|Default|SetPresentPlacement (+ (Variables|Default|GetPresentPlacement) DeltaSeconds)))
        (bind _aswt_progressbar (Utilities|Casting|CastToWT_Progressbar (UserInterface|GetUserWidgetObject (Variables|Default|GetProgressBar))))
        (Progress|SetPercent (Variables|/Game/Blueprints/UI/WT_Progressbar.WT_Progressbar_C|GetProgressBar_0 _aswt_progressbar) (/ _output_get 3.0))
        (if (>= (/ _output_get 3.0) 1.0)
          (Variables|Default|SetHasDeliveredPresent true)
          (Rendering|SetVisibility (Variables|Default|GetProgressBar) false false))
        (else
          (Variables|Default|SetPresentPlacement 0.0)
          (bind _aswt_progressbar_2 (Utilities|Casting|CastToWT_Progressbar (UserInterface|GetUserWidgetObject (Variables|Default|GetProgressBar))))
          (Progress|SetPercent (Variables|/Game/Blueprints/UI/WT_Progressbar.WT_Progressbar_C|GetProgressBar_0 _aswt_progressbar_2) 0.0))))))

(event Input|ActionEvents|InputActionSneak
  (params (Key :type Key%20Structure))
  (:Pressed
    (Variables|Default|SetSneaking true))
  (:Released
    (Variables|Default|SetSneaking false)))

(event Input|ActionEvents|InputActionAction
  (params (Key :type Key%20Structure))
  (:Pressed
    (if (Variables|Default|GetIsNearTree)
      (Variables|Default|SetIsPlacing true)))
  (:Released
    (Variables|Default|SetIsPlacing false)))

(event Input|AxisEvents|InputAxisMoveForward
  (params (AxisValue :type Float%20%28single-precision%29))
  (bind _returnvalue (Pawn|GetControlRotation :!class /Script/Engine.Pawn))
  (bind _returnvalue_2 (Transformation|GetActorLocation))
  (bind _pitch (Math|Rotator|BreakRotator _returnvalue))
  (bind _returnvalue_3 (Math|Rotator|MakeRotator 0.0 _pitch 0.0))
  (bind _returnvalue_4 (Math|Vector|GetForwardVector _returnvalue_3))
  (if (Variables|Default|GetSneaking)
    (Variables|Default|SetForwardValue (* AxisValue 0.5))
    (else
      (Variables|Default|SetForwardValue AxisValue)))
  (Pawn|Input|AddMovementInput _returnvalue_4 (Variables|Default|GetForwardValue) false)
  (Variables|Default|SetSpeed (Math|Vector|VectorLength (+ (* _returnvalue_4 (Variables|Default|GetForwardValue)) (* (Math|Vector|GetRightVector _returnvalue_3) (Variables|Default|GetRightValue)))))
  (Development|PrintString (Utilities|String|ToString(Rotator) (Math|Rotator|FindLookatRotation _returnvalue_2 (+ _returnvalue_2 (+ (* _returnvalue_4 (Variables|Default|GetForwardValue)) (* (Math|Vector|GetRightVector _returnvalue_3) (Variables|Default|GetRightValue)))))))
  (Transformation|SetWorldRotation (Variables|Default|GetSantaMesh) (Math|Rotator|FindLookatRotation _returnvalue_2 (+ _returnvalue_2 (+ (* _returnvalue_4 (Variables|Default|GetForwardValue)) (* (Math|Vector|GetRightVector _returnvalue_3) (Variables|Default|GetRightValue))))) false false))

(event Input|AxisEvents|InputAxisMoveRight
  (params (AxisValue :type Float%20%28single-precision%29))
  (if (Variables|Default|GetSneaking)
    (Variables|Default|SetRightValue (* AxisValue 0.5))
    (else
      (Variables|Default|SetRightValue AxisValue)))
  (Pawn|Input|AddMovementInput (Math|Vector|GetRightVector (Math|Rotator|MakeRotator 0.0 (.Pitch (Math|Rotator|BreakRotator (Pawn|GetControlRotation :!class /Script/Engine.Pawn))) 0.0)) (Variables|Default|GetRightValue) false))

(event Input|KeyboardEvents|P
  (params (Key :type Key%20Structure))
  (:Pressed
    (bind _returnvalue (UserInterface|CreateWidget "/Game/Blueprints/UI/WT_GameOverScreen.WT_GameOverScreen_C"))
    (UserInterface|Viewport|AddtoViewport _returnvalue 0)
    (Variables|/Script/Engine.PlayerController|SetbShowMouseCursor (Game|GetPlayerController 0) true)
    (Game|SetGamePaused true)))

(fn ConstructionScript)